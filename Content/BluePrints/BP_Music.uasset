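; BP_Music is an interactable music player actor that starts a 2D music track at BeginPlay and lets interaction pause or resume it.
; The DInteract interface event flips the Playing flag, pauses the audio component accordingly and passes the flag to ChangeAnimation.
; ChangeAnimation turns the flag into a play rate, freezing or running both skeletal meshes.
; Cursor-over events on Reewr toggle custom depth on those meshes.
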(event `self.ReceiveBeginPlay`
  (bind _returnvalue (`GameplayStatics.SpawnSound2D` (`self.Music`) 1.0 1.0 0.0 null))
  (`ActorComponent.SetActive` _returnvalue true false)
  (set `self.Audio` _returnvalue)
  (set `self.Playing` true))

(event `self.Interactable.DInteract`
  (bind _output_get (set `self.Playing` (not (`self.Playing`))))
  (`AudioComponent.SetPaused` (`self.Audio`) (not _output_get))
  (`self.ChangeAnimation` _output_get))

(event `self.reewr.OnBeginCursorOver`
  (params (TouchedComponent :type "PrimitiveComponent Object Reference"))
  (for _array_element (`|MakeArray` (`self.SkeletalMesh`) (`self.SkeletalMesh1`))
    (`PrimitiveComponent.SetRenderCustomDepth` _array_element true)))

(event `self.reewr.OnEndCursorOver`
  (params (TouchedComponent :type "PrimitiveComponent Object Reference"))
  (for _array_element (`|MakeArray` (`self.SkeletalMesh`) (`self.SkeletalMesh1`))
    (`PrimitiveComponent.SetRenderCustomDepth` _array_element false)))

(fn `ChangeAnimation`
  (params (Enable :type Boolean))
  (bind _returnvalue (`KismetMathLibrary.Conv_BoolToDouble` Enable))
  (`SkeletalMeshComponent.SetPlayRate` (`self.SkeletalMesh`) _returnvalue)
  (`SkeletalMeshComponent.SetPlayRate` (`self.SkeletalMesh1`) _returnvalue))

(fn `UserConstructionScript`)