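; Blueprint function library of global helpers for a tavern game, covering tavern open/close, rewards, UI and input mode.
; Getters return the custom game instance, player character, tavern inventory component and tavern manager, mostly through casts or GetActorOfClass lookups.
; Reputation and money edits record rewards and update game instance totals, clamping reputation at zero, then push them to the manager's tavern widget.
; UI helpers update or reset every top-level tavern UI widget.
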(fn `CastToPlayerChar`
  (returns (Player :type "/Game/BluePrints/Character/BP_Character Object Reference"))
  (bind _asbp_character (cast `/Game/BluePrints/Character/BP_Character` (`GameplayStatics.GetPlayerCharacter` null)))
  (return _asbp_character))

(fn `CloseTavern`
  (bind _returnvalue (`GameplayStatics.GetActorOfClass` null "/Game/BluePrints/GameManaging/BP_TavernManager.BP_TavernManager_C"))
  (`/Game/BluePrints/GameManaging/BP_TavernManager.CloseTavernEvent` _returnvalue))

(fn `EditMoneyReward`
  (params (Amount :type Integer))
  (bind _gameinstance (`self.GetCustomGameInstance` null))
  (`/Game/BluePrints/GameManaging/BP_GameInstance.AddReward` _gameinstance Amount 0 0 0)
  (bind _output_get (set `/Game/BluePrints/GameManaging/BP_GameInstance.Money` (+ (`/Game/BluePrints/GameManaging/BP_GameInstance.Money` _gameinstance) Amount) _gameinstance))
  (cast `/Game/BluePrints/Character/BP_Character` (`GameplayStatics.GetPlayerCharacter` null))
  (bind _returnvalue (`GameplayStatics.GetActorOfClass` null "/Game/BluePrints/GameManaging/BP_TavernManager.BP_TavernManager_C"))
  (`/Game/BluePrints/UI/WB_TavernUI.GainMoney` (`/Game/BluePrints/GameManaging/BP_TavernManager.TavernWidget` _returnvalue) _output_get))

(fn `EditReputation`
  (params (Amount :type Integer))
  (bind _gameinstance (`self.GetCustomGameInstance` null))
  (`/Game/BluePrints/GameManaging/BP_GameInstance.AddReward` _gameinstance 0 Amount 0 0)
  (bind _output_get (set `/Game/BluePrints/GameManaging/BP_GameInstance.TavernReputation` (`KismetMathLibrary.Max` (+ (`/Game/BluePrints/GameManaging/BP_GameInstance.TavernReputation` _gameinstance) Amount)) _gameinstance))
  (cast `/Game/BluePrints/Character/BP_Character` (`GameplayStatics.GetPlayerCharacter` null))
  (bind _returnvalue (`GameplayStatics.GetActorOfClass` null "/Game/BluePrints/GameManaging/BP_TavernManager.BP_TavernManager_C"))
  (`/Game/BluePrints/UI/WB_TavernUI.UpdateReputation` (`/Game/BluePrints/GameManaging/BP_TavernManager.TavernWidget` _returnvalue) _output_get))

(fn `GetCustomGameInstance`
  (returns (GameInstance :type "/Game/BluePrints/GameManaging/BP_GameInstance Object Reference"))
  (bind _asbp_game_instance (cast `/Game/BluePrints/GameManaging/BP_GameInstance` (`GameplayStatics.GetGameInstance` null)))
  (return _asbp_game_instance))

(fn `GetTableManager`
  (returns (TableManager :type "/Game/BluePrints/GameManaging/BP_TavernManager Object Reference"))
  (bind _returnvalue (`GameplayStatics.GetActorOfClass` null "/Game/BluePrints/GameManaging/BP_TavernManager.BP_TavernManager_C"))
  (return _returnvalue))

(fn `GetTavernInventory`
  (returns (Inventory :type "/Game/BluePrints/ActorComponents/DrinksAndIngredientsInventory Object Reference"))
  (bind _player (`self.CastToPlayerChar` null))
  (return (`Actor.GetComponentByClass` _player "/Game/BluePrints/ActorComponents/DrinksAndIngredientsInventory.DrinksAndIngredientsInventory_C")))

(fn `OpenTavern`
  (bind _returnvalue (`GameplayStatics.GetActorOfClass` null "/Game/BluePrints/GameManaging/BP_TavernManager.BP_TavernManager_C"))
  (`/Game/BluePrints/GameManaging/BP_TavernManager.OpenTavern` _returnvalue))

(fn `ResetTavernUI`
  (bind _foundwidgets (`WidgetBlueprintLibrary.GetAllWidgetsOfClass` null "/Game/BluePrints/UI/WB_TavernUI.WB_TavernUI_C"))
  (for _array_element _foundwidgets
    (`/Game/BluePrints/UI/WB_TavernUI.Reset` _array_element)))

(fn `SetUIOnly`
  (`WidgetBlueprintLibrary.SetInputMode_UIOnlyEx` (`GameplayStatics.GetPlayerController` null) null))

(fn `UpdateTavernUI`
  (bind _foundwidgets (`WidgetBlueprintLibrary.GetAllWidgetsOfClass` null "/Game/BluePrints/UI/WB_TavernUI.WB_TavernUI_C"))
  (for _array_element _foundwidgets
    (`/Game/BluePrints/UI/WB_TavernUI.UpdateUI` _array_element)))