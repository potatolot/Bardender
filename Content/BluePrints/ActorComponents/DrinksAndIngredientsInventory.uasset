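; Actor component that holds drink and ingredient inventories for making and selling drinks.
; MakeDrink and SellDrink find a drink by NameID, adjust its quantity and debit or credit Money on the custom game instance at the same Cost.
; CompareMoney divides Money by a drink's cost to gauge affordability.
; UseIngredients only looks up ingredients without consuming them, and CreateNewDrink is an empty stub.
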(fn `CompareMoney`
  (params (NameID :type Name))
  (returns (QuantityAbleToBuy :type Integer))
  (bind _drink (`self.FindDrinkFromName` NameID))
  (bind _gameinstance (`/Game/BluePrints/FunctionLists/Global_Functions.GetCustomGameInstance`))
  (return (/ (`/Game/BluePrints/BP_GameInstance.Money` _gameinstance) (`.Cost_8_51A84966477FEEB720B79287B1C6F2C7` (break `/Game/BluePrints/ActorComponents/Struct_Drinks` _drink)))))

(fn `CreateNewDrink`
  (params (`Ingredient 1` :type Name) (`Ingredient 2` :type Name)))

(fn `FindDrinkFromName`
  (params (NameID :type Name))
  (returns (Drink :type "/Game/BluePrints/ActorComponents/Struct_Drinks Structure") (Index :type Integer))
  (for (_array_element _array_index) (`self.DrinkInventory`)
    (if (== NameID (`.NameID_9_D08DF0F14AFA6573831647ABBB2A35E7` (break `/Game/BluePrints/ActorComponents/Struct_Drinks` _array_element)))
      (return _array_element _array_index))))

(fn `FindIngredientFromName`
  (params (NameID :type Name))
  (returns (Ingredient :type "/Game/BluePrints/Ingredients/IngredientStructure Structure") (index :type Integer))
  (for (_array_element _array_index) (`self.IngredientInventory`)
    (if (== NameID (`.NameID_9_EA362C444500E16970580C8D557C9483` (break `/Game/BluePrints/Ingredients/IngredientStructure` _array_element)))
      (return _array_element _array_index))))

(fn `GetDrinkQuantity`
  (params (NameID :type Name))
  (returns (Quantity :type Integer))
  (bind _drink (`self.FindDrinkFromName` NameID))
  (return (`.Quantity_6_38BFDB0E491F8E64F1814D9133F8677E` (break `/Game/BluePrints/ActorComponents/Struct_Drinks` _drink))))

(fn `MakeDrink`
  (params (NameID :type Name) (Quantity :type Integer))
  (bind (_drink _index) (`self.FindDrinkFromName` NameID))
  (bind (_nameid _quantity _cost _ingredientids) (break `/Game/BluePrints/ActorComponents/Struct_Drinks` _drink))
  (`self.UpdateMoney` _cost Quantity)
  (`KismetArrayLibrary.Array_Set` (`self.DrinkInventory`) _index (make `/Game/BluePrints/ActorComponents/Struct_Drinks` _nameid (+ _quantity Quantity) _cost _ingredientids)))

(fn `SellDrink`
  (params (NameID :type Name) (Quantity :type Integer))
  (bind (_drink _index) (`self.FindDrinkFromName` NameID))
  (bind (_nameid _quantity _cost _ingredientids) (break `/Game/BluePrints/ActorComponents/Struct_Drinks` _drink))
  (`self.UpdateMoney` (* _cost -1) Quantity)
  (`KismetArrayLibrary.Array_Set` (`self.DrinkInventory`) _index (make `/Game/BluePrints/ActorComponents/Struct_Drinks` _nameid (- _quantity Quantity) _cost _ingredientids)))

(fn `UpdateMoney`
  (params (Cost :type Integer) (Quantity :type Integer))
  (bind _gameinstance (`/Game/BluePrints/FunctionLists/Global_Functions.GetCustomGameInstance`))
  (set `/Game/BluePrints/BP_GameInstance.Money` (- (`/Game/BluePrints/BP_GameInstance.Money` _gameinstance) (* Cost Quantity)) _gameinstance))

(fn `UseIngredients`
  (params (NameID :type Name))
  (returns (ReducedCost :type Integer))
  (bind _drink (`self.FindDrinkFromName` NameID))
  (for _array_element (`.IngredientIDs_14_F9A209C04583CDA366C7258465AA32DD` (break `/Game/BluePrints/ActorComponents/Struct_Drinks` _drink))
    (bind _ingredient (`self.FindIngredientFromName` _array_element))))