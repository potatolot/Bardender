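; Wall_Change is an actor component that toggles its owner's static mesh visibility based on the camera's viewing direction, apparently for walls.
; On BeginPlay it caches the level's CameraActor.
; Each Tick it dots the camera's horizontal forward vector with the mesh's right vector.
; The mesh shows only when that value lies strictly between -1 and -0.5, so it hides otherwise, including when exactly opposed.
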(event `self.ReceiveBeginPlay`
  (bind _returnvalue (`GameplayStatics.GetActorOfClass` "/Script/Engine.CameraActor"))
  (set `self.Camera` _returnvalue))

(event `self.ReceiveTick`
  (params (DeltaSeconds :type "Float (single-precision)"))
  (bind _returnvalue (`Actor.GetComponentByClass` (`self.GetOwner`) "/Script/Engine.StaticMeshComponent"))
  (bind _returnvalue_2 (`KismetMathLibrary.Dot_VectorVector` (`KismetMathLibrary.Normal` (`KismetMathLibrary.MakeVector` (.x (`SceneComponent.GetForwardVector` (`Actor.RootComponent` (`self.Camera`)))) (.y (`SceneComponent.GetForwardVector` (`Actor.RootComponent` (`self.Camera`)))))) (`KismetMathLibrary.Normal` (`SceneComponent.GetRightVector` _returnvalue))))
  (if (and (< _returnvalue_2 -0.5) (> _returnvalue_2 -1.0))
    (`SceneComponent.SetVisibility` _returnvalue true false)
    (else
      (`SceneComponent.SetVisibility` _returnvalue false false))))