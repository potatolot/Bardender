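; Tavern manager that seats groups of AI customers at tables while the tavern runs.
; Opening shows the tavern UI, then a randomly re-armed timer spawns groups until free tables or the game instance's expected customers run out.
; Each group claims a random table, reduces the expected count and receives seat locations at spawn.
; Emptying a table only tells it to leave; closing also moves tables back to available while iterating the taken list.
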(event `self.ReceiveBeginPlay`
  ;[1 1 1] Initialize Widgets
  (bind _outactors (`GameplayStatics.GetAllActorsOfClass` "/Game/BluePrints/Tavern_Logic/BP_Table.BP_Table_C"))
  (set `self.AvailableTables` _outactors)
  (bind _returnvalue (`|CreateWidget` "/Game/BluePrints/UI/WB_TavernUI.WB_TavernUI_C"))
  (set `self.TavernWidget` _returnvalue))

(event `OpenTavern`
  ;[1 1 1] Add tavern widget to screen
  (set `self.TavernOpened` true)
  (`UserWidget.AddToViewport` (`self.TavernWidget`) 0)
  (`KismetSystemLibrary.Delay` 5.0)
  (`self.FillNewTable`))

(event `FillNewTable`
  ;[1 1 1] Check if any tables are available
  (if (> (`KismetArrayLibrary.Array_Length` (`self.AvailableTables`)) 0)
    ;[1 1 1] Check if any customers are left
    (bind _gameinstance (`/Game/BluePrints/FunctionLists/Global_Functions.GetCustomGameInstance`))
    (if (> (`/Game/BluePrints/GameManaging/BP_GameInstance.ExpectedCustomers` _gameinstance) 0)
      (`self.SpawnNewGroup`)
      (`KismetSystemLibrary.K2_SetTimerDelegate` (delegate `FillNewTable`) (`KismetMathLibrary.RandomFloatInRange` 2.0 5.0)))))

(fn `CloseTavern`
  (bind _takentables (`self.TakenTables`))
  (for _array_element _takentables
    (`/Game/BluePrints/Tavern_Logic/BP_Table.LeaveTavern` _array_element)
    (`KismetArrayLibrary.Array_Add` (`self.AvailableTables`) _array_element)
    (`KismetArrayLibrary.Array_RemoveItem` _takentables _array_element)))

(fn `EmptyOutTable`
  (params (TableNumber :type Integer))
  (for _array_element (`self.TakenTables`)
    (if (== TableNumber (`/Game/BluePrints/Tavern_Logic/BP_Table.TableNumber` _array_element))
      ;[1 1 1] Table leave
      (`/Game/BluePrints/Tavern_Logic/BP_Table.LeaveTavern` _array_element))))

(fn `GetOrderTable`
  (params (TableNumber :type Integer)))

(fn `GetRandomCustomerNumberForTable`
  (returns (CustomerNumber :type Integer))
  (bind _gameinstance (`/Game/BluePrints/FunctionLists/Global_Functions.GetCustomGameInstance`))
  (bind _output_get (set `self.RandomNumber` (`KismetMathLibrary.RandomIntegerInRange` 1 (`KismetMathLibrary.Clamp` (`/Game/BluePrints/GameManaging/BP_GameInstance.ExpectedCustomers` _gameinstance) 1 4))))
  (`/Game/BluePrints/GameManaging/BP_GameInstance.DecreaseExpectedCustomers` _gameinstance _output_get)
  (`/Game/BluePrints/UI/WB_TavernUI.UpdateCustomerNumber` (`self.TavernWidget`))
  (`KismetSystemLibrary.PrintString` (`KismetStringLibrary.Conv_IntToString` _output_get))
  (return _output_get))

(fn `SetRandomSpawnTime`
  (set `self.SpawnTime` (`KismetMathLibrary.RandomIntegerInRange` 2 5)))

(fn `SpawnNewGroup`
  (bind _takentables (`self.TakenTables`))
  (bind _availabletables (`self.AvailableTables`))
  (bind _returnvalue (`KismetArrayLibrary.Array_Length` (`self.AvailableTables`)))
  (bind _returnvalue_2 (`self.GetTransform` (`self.SpawnPoint`)))
  (bind _output (`|GetArrayItem` _takentables (`KismetArrayLibrary.Array_LastIndex` _takentables)))
  (if (< 0 _returnvalue)
    (bind _output_get (set `self.RandomTable` (`KismetMathLibrary.RandomIntegerInRange` 0 (- _returnvalue 1))))
    (bind _output_2 (`|GetArrayItem` _availabletables _output_get))
    (`/Game/BluePrints/Tavern_Logic/BP_Table.SetAvailability` _output_2 false)
    (`KismetArrayLibrary.Array_Add` (`self.TakenTables`) _output_2)
    (`KismetArrayLibrary.Array_RemoveItem` _availabletables _output_2)
    (bind _customernumber (`self.GetRandomCustomerNumberForTable`))
    (for _index (range 1 (+ _customernumber 1))
      ;[1 1 1] TO DO: Spawn amount of new ai characters at spawnpoint
      (bind _location (`/Game/BluePrints/Tavern_Logic/BP_Table.GetSitLocation` _output _index))
      (bind _returnvalue_3 (`|SpawnActorFromClass` (`KismetArrayLibrary.Array_Random` (`self.AICharacters`)) _returnvalue_2 "Undefined" "OverrideRootScale" null _location _returnvalue_2 null))
      (`KismetArrayLibrary.Array_Add` (`/Game/BluePrints/Tavern_Logic/BP_Table.NPCList` _output) _returnvalue_3))))

(fn `UserConstructionScript`)