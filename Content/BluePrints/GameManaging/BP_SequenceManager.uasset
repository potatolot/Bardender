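; BP_SequenceManager runs the game's opening dialogue sequence on BeginPlay.
; It creates a WB_MainDialogue widget, adds it to the viewport and keeps a reference to it.
; StartBeginSequence then switches the player to UI-only input without mouse lock, passes the StartDialog text to the widget and calls ContinueDialog to begin the dialogue.
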(event `self.ReceiveBeginPlay`
  (bind _returnvalue (`|CreateWidget` "/Game/BluePrints/UI/WB_MainDialogue.WB_MainDialogue_C"))
  (bind _output_get (set `self.DialogueWidget` _returnvalue))
  (`UserWidget.AddToViewport` _output_get 0)
  (`self.StartBeginSequence`))

(event `StartBeginSequence`
  (bind _dialoguewidget (`self.DialogueWidget`))
  (`WidgetBlueprintLibrary.SetInputMode_UIOnlyEx` (`GameplayStatics.GetPlayerController` 0) null)
  (set `/Game/BluePrints/UI/WB_MainDialogue.DialogueText` (`self.StartDialog`) _dialoguewidget)
  (`/Game/BluePrints/UI/WB_MainDialogue.ContinueDialog` _dialoguewidget))

(fn `UserConstructionScript`)