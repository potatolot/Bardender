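; BP_BarFinal is an interactable bar actor that opens the bar UI when the player interacts with it.
; On BeginPlay it creates a WB_BarUI widget and passes it a reference to itself.
; Hovering the cursor over the bar mesh toggles highlighting on the root component.
; Interaction adds the widget to the viewport in UI-only input mode and starts its tutorial if TutorialCompleted is false.
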(event `self.ReceiveBeginPlay`
  (bind _returnvalue (`|CreateWidget` "/Game/BluePrints/UI/WB_BarUI.WB_BarUI_C" (`GameplayStatics.GetPlayerController` 0)))
  (bind _output_get (set `self.BarUI` _returnvalue))
  (set `/Game/BluePrints/UI/WB_BarUI.BarReference` self _output_get))

(event `self.ReceiveTick`
  (params (DeltaSeconds :type "Float (single-precision)")))

(event `self.BarMesh.OnBeginCursorOver`
  (params (TouchedComponent :type "PrimitiveComponent Object Reference"))
  (`/Game/BluePrints/FunctionLists/FL_Interactable.Highlighted` (`self.DefaultSceneRoot`)))

(event `self.BarMesh.OnEndCursorOver`
  (params (TouchedComponent :type "PrimitiveComponent Object Reference"))
  (`/Game/BluePrints/FunctionLists/FL_Interactable.DeHighlight` (`self.DefaultSceneRoot`)))

(event `self.Interactable.DInteract`
  (bind _barui (`self.BarUI`))
  (`UserWidget.AddToViewport` _barui 0)
  (`WidgetBlueprintLibrary.SetInputMode_UIOnlyEx` (`GameplayStatics.GetPlayerController` 0) _barui)
  (if (not (`self.TutorialCompleted`))
    (`/Game/BluePrints/UI/WB_BarUI.StartTutorial` _barui)))

(fn `UserConstructionScript`)