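; Player-controlled 2D flipbook character for the dungeon minigame that runs, jumps and shoots.
; Movement input and falling state pick idle, run or jump flipbooks, with negative X scale mirroring the sprite.
; Attacking blocks move and jump input, spawns a bullet at the mesh and faces the sprite toward the mouse's screen half.
; HIT flashes damage by toggling a dynamic material's Hit parameter around a short delay.
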(event `HIT`
  (bind _returnvalue (`PrimitiveComponent.CreateDynamicMaterialInstance` (`self.PaperFlipbook`) 0 "/Game/Art/DungeonMiniGame/Mat_Enemies.Mat_Enemies" "None"))
  (`MaterialInstanceDynamic.SetScalarParameterValue` _returnvalue "Hit" 0.0)
  (`PrimitiveComponent.SetMaterial` (`self.PaperFlipbook`) 0 _returnvalue)
  (`KismetSystemLibrary.Delay` 0.5)
  (bind _returnvalue_2 (`PrimitiveComponent.CreateDynamicMaterialInstance` (`self.PaperFlipbook`) 0 "/Game/Art/DungeonMiniGame/Mat_Enemies.Mat_Enemies" "None"))
  (`MaterialInstanceDynamic.SetScalarParameterValue` _returnvalue_2 "Hit" 1.0)
  (`PrimitiveComponent.SetMaterial` (`self.PaperFlipbook`) 0 _returnvalue_2))

(event `self.ReceiveTick`
  (params (DeltaSeconds :type "Float (single-precision)"))
  (if (`NavMovementComponent.IsFalling` (`self.CharacterMovement`))
    (`PaperFlipbookComponent.SetFlipbook` (`self.PaperFlipbook`) (`self.FBJump`))))

(event `InputAxis|MoveRight`
  (params (AxisValue :type "Float (single-precision)"))
  (if (`self.Attacking`)
    _
    (elif (== AxisValue 0.0)
      (`PaperFlipbookComponent.SetFlipbook` (`self.PaperFlipbook`) (`self.FBIdle`))
      (else
        (`self.AddMovementInput` (1.0 0.0 0.0) AxisValue)
        (`PaperFlipbookComponent.SetFlipbook` (`self.PaperFlipbook`) (`self.FBRun`))
        (if (< AxisValue 0.0)
          (`SceneComponent.SetRelativeScale3D` (`self.PaperFlipbook`) (-0.5 0.5 0.5))
          (else
            (`SceneComponent.SetRelativeScale3D` (`self.PaperFlipbook`) (0.5 0.5 0.5))))))))

(event `InputAction|Jump`
  (params (Key :type "Key Structure"))
  (:`Pressed`
    (if (not (`self.Attacking`))
      (`self.Jump`)))
  (:`Released`
    (`self.StopJumping`)))

(event `InputAction|Attack`
  (params (Key :type "Key Structure"))
  (:`Pressed`
    (set `self.Attacking` true)
    (`PaperFlipbookComponent.SetFlipbook` (`self.PaperFlipbook`) (`self.FBAttack`))
    ;[1 1 1] Shoot Logic
    (`|SpawnActorFromClass` "/Game/BluePrints/DungeonMiniGame/Bullet.Bullet_C" (`KismetMathLibrary.MakeTransform` (`SceneComponent.K2_GetComponentLocation` (`self.Mesh`)) (struct) (0.3 0.3 0.3)) "Undefined" "OverrideRootScale" null null)
    (`SceneComponent.SetRelativeScale3D` (`self.PaperFlipbook`) (`KismetMathLibrary.MakeVector` (* (`KismetMathLibrary.SignOfFloat` (- (/ (`PlayerController.GetMousePosition` (`GameplayStatics.GetPlayerController` 0)) (`KismetMathLibrary.BreakVector2D` (`WidgetLayoutLibrary.GetViewportSize`))) 0.5)) 0.5) 0.5 0.5)))
  (:`Released`
    (set `self.Attacking` false)))

(fn `UserConstructionScript`)