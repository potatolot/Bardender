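; Enemy class for the dungeon minigame: a sprite that patrols back and forth along world X and hurts the 2D character on overlap.
; A sine of its lifetime drives both movement input and the sprite's horizontal flip.
; Bullet overlaps toggle a Hit parameter through dynamic material instances for a brief flash.
; Health drops only after that delay, and the actor is destroyed at zero.
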(event `self.ReceiveBeginPlay`
  (set `self.BeginLoc` (`SceneComponent.K2_GetComponentLocation` (`self.Sprite`))))

(event `self.ReceiveTick`
  (params (DeltaSeconds :type "Float (single-precision)"))
  (bind _sprite (`self.Sprite`))
  (bind (_returnvalue_x _returnvalue_y _returnvalue_z) (`KismetMathLibrary.BreakVector` (`SceneComponent.K2_GetComponentScale` _sprite)))
  (bind _returnvalue (* (`KismetMathLibrary.Sin` (`self.GetGameTimeSinceCreation`)) 0.5))
  (`self.AddMovementInput` (1.0 0.0 0.0) _returnvalue)
  (`SceneComponent.SetWorldScale3D` _sprite (`KismetMathLibrary.MakeVector` (`KismetMathLibrary.SignOfFloat` _returnvalue) _returnvalue_y _returnvalue_z)))

(event `self.ReceiveActorBeginOverlap`
  (params (OtherActor :type "Actor Object Reference"))
  (cast `/Game/BluePrints/DungeonMiniGame/Bullet` OtherActor
    (:`then`
      (bind _returnvalue (`PrimitiveComponent.CreateDynamicMaterialInstance` (`self.Sprite`) 0 "/Game/Art/DungeonMiniGame/Mat_Enemies.Mat_Enemies" "None"))
      (`MaterialInstanceDynamic.SetScalarParameterValue` _returnvalue "Hit" 0.0)
      (`PrimitiveComponent.SetMaterial` (`self.Sprite`) 0 _returnvalue)
      (`KismetSystemLibrary.Delay` 0.5)
      (bind _returnvalue_2 (`PrimitiveComponent.CreateDynamicMaterialInstance` (`self.Sprite`) 0 "/Game/Art/DungeonMiniGame/Mat_Enemies.Mat_Enemies" "None"))
      (`MaterialInstanceDynamic.SetScalarParameterValue` _returnvalue_2 "Hit" 1.0)
      (`PrimitiveComponent.SetMaterial` (`self.Sprite`) 0 _returnvalue_2)
      (`self.HIT`))
    (:`CastFailed`
      (bind _as2dcharacter (cast `/Game/BluePrints/DungeonMiniGame/2DCharacter` OtherActor))
      (`/Game/BluePrints/DungeonMiniGame/2DCharacter.HIT` _as2dcharacter))))

(event `HIT`
  (bind _result (`/Engine/EditorBlueprintResources/StandardMacros.DecrementInt` (`self.Health`))
    (:`  `
      (if (<= _result 0)
        (`self.K2_DestroyActor`)))))

(fn `UserConstructionScript`)