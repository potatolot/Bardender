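; Bullet is a projectile actor in the dungeon minigame that flies left or right along the X axis.
; On BeginPlay it sets its ProjectileMovement velocity to a fixed speed, signed by whether the mouse cursor is on the left or right half of the viewport.
; It also prints the cursor's X position, then destroys itself after a short delay, with no overlap or hit logic.
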(event `self.ReceiveBeginPlay`
  (bind _locationx (`PlayerController.GetMousePosition` (`GameplayStatics.GetPlayerController` 0)))
  (`KismetSystemLibrary.PrintString` (`KismetStringLibrary.Conv_DoubleToString` _locationx))
  (set `MovementComponent.Velocity` (* (200.0 0.0 0.0) (`KismetMathLibrary.SignOfFloat` (- (/ _locationx (`KismetMathLibrary.BreakVector2D` (`WidgetLayoutLibrary.GetViewportSize`))) 0.5))) (`self.ProjectileMovement`))
  (`KismetSystemLibrary.Delay` 1.0)
  (`self.K2_DestroyActor`))

(fn `UserConstructionScript`)