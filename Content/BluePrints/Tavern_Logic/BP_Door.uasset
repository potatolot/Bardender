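; Tavern door actor that lets the player open and close the tavern through a confirmation widget, with highlight and interaction blocked while the game state is Closed.
; The widget's button moves the game instance from Preparing to Open, updating expected customers, or from Open to Closed, showing the end-of-day overview.
; ChangeToState refreshes button text and dialogue, including a customer forecast capped by the tavern inventory's total drinks.
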(event `self.Box.OnBeginCursorOver`
  (params (TouchedComponent :type "PrimitiveComponent Object Reference"))
  (`self.CheckGameState`
    (:`Open`
      (if (`/Game/BluePrints/ActorComponents/Interactable.Active` (`self.Interactable`))
        (`/Game/BluePrints/FunctionLists/FL_Interactable.Highlighted` (`self.DefaultSceneRoot`))))))

(event `self.Box.OnEndCursorOver`
  (params (TouchedComponent :type "PrimitiveComponent Object Reference"))
  (`self.CheckGameState`
    (:`Open`
      (if (`/Game/BluePrints/ActorComponents/Interactable.Active` (`self.Interactable`))
        (`/Game/BluePrints/FunctionLists/FL_Interactable.DeHighlight` (`self.DefaultSceneRoot`))))))

(event `self.ReceiveBeginPlay`
  (bind _returnvalue (`|CreateWidget` "/Game/BluePrints/UI/WB_ChoiceUI.WB_ChoiceUI_C"))
  (bind _output_get (set `self.DoorWidget` _returnvalue))
  (bind _returnvalue_2 (`|CreateWidget` "/Game/BluePrints/UI/WB_OverviewDayEnd.WB_OverviewDayEnd_C"))
  (set `self.EndOfDayWidget` _returnvalue_2)
  (add `/Game/BluePrints/UI/WB_ChoiceUI.Callbutton` _output_get (delegate `ButtonLogic`))
  (`self.ChangeToState` "NewEnumerator2"))

(event `ButtonLogic`
  (bind _doorwidget (`self.DoorWidget`))
  (bind _gameinstance (`/Game/BluePrints/FunctionLists/Functions.GetCustomGameInstance`))
  (switch `/Game/BluePrints/GameManaging/EGameState` (`/Game/BluePrints/GameManaging/BP_GameInstance.GameState` _gameinstance)
    (:`NewEnumerator0`
      ;[1 1 1] Close -> Open
      (bind _gameinstance_2 (`/Game/BluePrints/FunctionLists/Functions.GetCustomGameInstance`))
      (`/Game/BluePrints/GameManaging/BP_GameInstance.UpdateExpectedCustomers` _gameinstance_2)
      (`WidgetBlueprintLibrary.SetInputMode_GameAndUIEx` (`GameplayStatics.GetPlayerController` 0) null "DoNotLock" false)
      (bind _gameinstance_3 (`/Game/BluePrints/FunctionLists/Functions.GetCustomGameInstance`))
      (bind _gamestate (`/Game/BluePrints/GameManaging/BP_GameInstance.ChangeGameState` _gameinstance_3 "NewEnumerator1"))
      (`self.ChangeToState` _gamestate)
      (`Widget.RemoveFromParent` _doorwidget))
    (:`NewEnumerator1`
      ;[1 1 1] Open -> Close
      (bind _gameinstance_4 (`/Game/BluePrints/FunctionLists/Functions.GetCustomGameInstance`))
      (bind _gamestate_2 (`/Game/BluePrints/GameManaging/BP_GameInstance.ChangeGameState` _gameinstance_4 "NewEnumerator2"))
      (`self.ChangeToState` _gamestate_2)
      (`UserWidget.AddToViewport` (`self.EndOfDayWidget`) 0)
      (`Widget.RemoveFromParent` _doorwidget))))

(event `self.Interactable.DInteract`
  (`self.CheckGameState`
    (:`Open`
      (`UserWidget.AddToViewport` (`self.DoorWidget`) 0)
      (`WidgetBlueprintLibrary.SetInputMode_UIOnlyEx` (`GameplayStatics.GetPlayerController` 0) null))))

(fn `ChangeToState`
  (params (NewParam :type "/Game/BluePrints/GameManaging/EGameState Enum" :default "NewEnumerator0"))
  (bind _doorwidget (`self.DoorWidget`))
  (bind _open (`/Game/BluePrints/UI/WB_ChoiceUI.Open` _doorwidget))
  (bind _buttontext (`/Game/BluePrints/UI/WB_ChoiceUI.ButtonText` _doorwidget))
  (switch `/Game/BluePrints/GameManaging/EGameState` NewParam
    (:`NewEnumerator0`
      (`Widget.SetVisibility` _open "Hidden")
      (`/Game/BluePrints/UI/WB_ChoiceUI.SetDialogue` _doorwidget "Are you sure you want to close down?" :!label _label))
    (:`NewEnumerator1`
      (`TextBlock.SetText` _buttontext "Close")
      (goto _label))
    (:`NewEnumerator2`
      (`Widget.SetVisibility` _open "Visible")
      (`TextBlock.SetText` _buttontext "Open")
      (`self.SetExpectedCustomers`))))

(fn `SetExpectedCustomers`
  (bind _gameinstance (`/Game/BluePrints/FunctionLists/Functions.GetCustomGameInstance`))
  (bind _inventory (`/Game/BluePrints/FunctionLists/Functions.GetTavernInventory`))
  (bind _totaldrinks (`/Game/BluePrints/ActorComponents/DrinksAndIngredientsInventory.TotalDrinks` _inventory))
  (`KismetSystemLibrary.PrintString` (`KismetStringLibrary.Conv_IntToString` _totaldrinks))
  (`/Game/BluePrints/UI/WB_ChoiceUI.SetDialogue` (`self.DoorWidget`) (`|FormatText` "You can expect {0} customers. Are you sure you are done preparing?" (`KismetMathLibrary.Clamp` _totaldrinks 0 (`/Game/BluePrints/GameManaging/BP_GameInstance.ExpectedCustomers` _gameinstance)))))

(fn `UserConstructionScript`)