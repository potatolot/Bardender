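; Interactable tavern bed that lets the player end the day and start a new one.
; Interacting branches on the game instance's GameState: PREPARING or OPEN shows a "not time to sleep" dialogue, while CLOSED offers a "Go Sleep" choice.
; Choosing sleep plays a rooster sound, calls ResetDay on the game instance and runs a fade widget animation before restoring game input.
; Cursor hover over the mesh toggles highlighting.
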(event `self.ReceiveBeginPlay`
  (bind _returnvalue (`|CreateWidget` "/Game/BluePrints/UI/WB_FadeOut.WB_FadeOut_C"))
  (set `self.FadeInOut` _returnvalue)
  (bind _returnvalue_2 (`|CreateWidget` "/Game/BluePrints/UI/WB_MainDialogue.WB_MainDialogue_C"))
  (set `self.DialogWidget` _returnvalue_2)
  (bind _returnvalue_3 (`|CreateWidget` "/Game/BluePrints/UI/WB_ChoiceUI.WB_ChoiceUI_C"))
  (bind _output_get (set `self.ChoiceWidget` _returnvalue_3))
  (`TextBlock.SetText` (`/Game/BluePrints/UI/WB_ChoiceUI.ButtonText` _output_get) "Go Sleep")
  (add `/Game/BluePrints/UI/WB_ChoiceUI.Callbutton` (`self.ChoiceWidget`) (delegate `GoToSleep`)))

(event `GoToSleep`
  (bind _fadeinout (`self.FadeInOut`))
  (`GameplayStatics.PlaySound2D` "/Game/Sounds/RoosterSound.RoosterSound" 1.0 1.0 0.0 null null)
  (`Widget.RemoveFromParent` (`self.ChoiceWidget`))
  (`WidgetBlueprintLibrary.SetInputMode_UIOnlyEx` (`GameplayStatics.GetPlayerController` 0) null)
  (bind _gameinstance (`/Game/BluePrints/FunctionLists/Functions.GetCustomGameInstance`))
  (`/Game/BluePrints/GameManaging/BP_GameInstance.ResetDay` _gameinstance)
  (`UserWidget.AddToViewport` _fadeinout 0)
  (`|PlayAnimation` _fadeinout (`/Game/BluePrints/UI/WB_FadeOut.Fadeinout` _fadeinout)
    (:`Finished`
      (`Widget.RemoveFromParent` _fadeinout)
      (`WidgetBlueprintLibrary.SetInputMode_GameAndUIEx` (`GameplayStatics.GetPlayerController` 0) null "DoNotLock" false))))

(event `self.StaticMesh.OnBeginCursorOver`
  (params (TouchedComponent :type "PrimitiveComponent Object Reference"))
  ;[1 1 1] InteractionLogic
  (`/Game/BluePrints/FunctionLists/FL_Interactable.Highlighted` (`self.DefaultSceneRoot`)))

(event `self.StaticMesh.OnEndCursorOver`
  (params (TouchedComponent :type "PrimitiveComponent Object Reference"))
  ;[1 1 1] InteractionLogic
  (`/Game/BluePrints/FunctionLists/FL_Interactable.DeHighlight` (`self.DefaultSceneRoot`)))

(event `self.Interactable.DInteract`
  ;[1 1 1] InteractionLogic
  (bind _gameinstance (`/Game/BluePrints/FunctionLists/Functions.GetCustomGameInstance`))
  (switch `/Game/BluePrints/GameManaging/EGameState` (`/Game/BluePrints/GameManaging/BP_GameInstance.GameState` _gameinstance)
    (:`NewEnumerator0`
      (`UserWidget.AddToViewport` (`self.DialogWidget`) 0 :!label _label)
      (`WidgetBlueprintLibrary.SetInputMode_UIOnlyEx` (`GameplayStatics.GetPlayerController` 0) null)
      (`TextBlock.SetText` (`/Game/BluePrints/UI/WB_MainDialogue.Dialogue` (`self.DialogWidget`)) "I don't think it's time to sleep yet"))
    (:`NewEnumerator1`
      (goto _label))
    (:`NewEnumerator2`
      (`UserWidget.AddToViewport` (`self.ChoiceWidget`) 0)
      (`WidgetBlueprintLibrary.SetInputMode_UIOnlyEx` (`GameplayStatics.GetPlayerController` 0) null)
      (`TextBlock.SetText` (`/Game/BluePrints/UI/WB_ChoiceUI.Dialogue` (`self.ChoiceWidget`)) "Ready to start a new day?"))))

(fn `UserConstructionScript`)