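; Tavern table actor that runs a seated NPC party's cycle of ordering, waiting, drinking and leaving.
; Timers drive the order prompt and wait tracking, switching world indicators, and pause while the interaction widget is open.
; OnOrder picks random drinks and registers with BP_Bar; BP_TavernManager empties the table after drinking or an overlong wait for service.
; ClearTable sends NPCs away, awarding money and reputation if served, otherwise deducting reputation.
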(event `SetAvailability`
  (params (newAvailability :type Boolean))
  ;[1 1 1] Set availability of Table
  (bind _output_get (set `/Game/BluePrints/ActorComponents/Interactable.Active` (not newAvailability) (`self.Interactable`)))
  (if _output_get
    ;;[1 1 1] Random order timer
    (if (not newAvailability)
      (bind _returnvalue (`KismetSystemLibrary.K2_SetTimerDelegate` (delegate `event`) (`KismetMathLibrary.RandomFloatInRange` 1.0 5.0)))
      (`KismetArrayLibrary.Array_Add` (`self.TimerHandels`) _returnvalue))
    (else
      (`self.ChangeIndicator` false)
      (set `self.ReadyToOrder` false))))

(event `event`
  ;[1 1 1] Set availability of Table
  ;;[1 1 1] Random order timer
  (`self.ChangeIndicator` false true)
  (set `self.ReadyToOrder` true)
  (set `self.OrderStatus` "NewEnumerator2")
  (set `self.WaitingTime` 0.0)
  ;[1 1 1] Comment
  (bind _returnvalue (`KismetSystemLibrary.K2_SetTimerDelegate` (delegate `WaitingToOrder`) 0.001 true))
  (`KismetArrayLibrary.Array_Add` (`self.TimerHandels`) _returnvalue))

(event `WaitingToOrder`
  (bind _returnvalue (+ (`self.WaitingTime`) 0.001))
  (if (`self.ReadyToOrder`)
    (set `self.WaitingTime` _returnvalue)
    (if (< (* (`self.MaxWaitingTime`) 0.66) _returnvalue)
      (`self.ChangeIndicator` false false true))
    (else
      (`KismetSystemLibrary.K2_ClearAndInvalidateTimerHandle` (stale `event` _returnvalue))
      (`KismetArrayLibrary.Array_RemoveItem` (`self.TimerHandels`) (stale `event` _returnvalue)))))

(event `OnOrder`
  (bind _drinkordersvar (`self.DrinkOrdersVar`))
  (bind _inventory (`/Game/BluePrints/FunctionLists/Functions.GetTavernInventory`))
  (set `self.DrinkOrdersVar` (`/Game/BluePrints/ActorComponents/DrinksAndIngredientsInventory.DrinkList` _inventory))
  ;[1 1 1] Generate Random Order
  (for _ (range (`KismetArrayLibrary.Array_Length` (`self.NPCList`)))
    (bind _output_get (set `self.CurrentOrder` (`KismetArrayLibrary.Array_Random` _drinkordersvar)))
    (`KismetArrayLibrary.Array_Add` (`self.Order`) _output_get)
    (`KismetArrayLibrary.Array_RemoveItem` _drinkordersvar _output_get))
  (bind _returnvalue (`GameplayStatics.GetActorOfClass` "/Game/BluePrints/Tavern_Logic/BP_Bar.BP_Bar_C"))
  (`/Game/BluePrints/Tavern_Logic/BP_Bar.AddNewOrder` _returnvalue self)
  (set `self.OrderStatus` "NewEnumerator1")
  (`self.ChangeIndicator` true)
  (set `self.ReadyToOrder` false)
  (set `self.WaitingTime` 0.0)
  ;[1 1 1] Comment
  (bind _returnvalue_2 (`KismetSystemLibrary.K2_SetTimerDelegate` (delegate `Awaiting order`) 0.001 true))
  (`KismetArrayLibrary.Array_Add` (`self.TimerHandels`) _returnvalue_2)
  (`self.PauseTimers`))

(event `Awaiting order`
  (bind _returnvalue (+ (`self.WaitingTime`) 0.001))
  (if (`self.Served`)
    (`self.ChangeIndicator` false)
    (`KismetSystemLibrary.K2_ClearAndInvalidateTimerHandle` (stale `OnOrder` _returnvalue_2))
    (`KismetArrayLibrary.Array_RemoveItem` (`self.TimerHandels`) (stale `OnOrder` _returnvalue_2))
    (else
      (set `self.WaitingTime` _returnvalue)
      (if (< (* (`self.MaxWaitingTime`) 0.66) _returnvalue)
        (`self.ChangeIndicator` false false true)
        (if (> (`self.WaitingTime`) (`self.MaxWaitingTime`))
          (`KismetSystemLibrary.K2_ClearAndInvalidateTimerHandle` (stale `OnOrder` _returnvalue_2))
          (`KismetArrayLibrary.Array_RemoveItem` (`self.TimerHandels`) (stale `OnOrder` _returnvalue_2))
          (bind _returnvalue_2 (`GameplayStatics.GetActorOfClass` "/Game/BluePrints/GameManaging/BP_TavernManager.BP_TavernManager_C"))
          (`/Game/BluePrints/GameManaging/BP_TavernManager.EmptyOutTable` _returnvalue_2 (`self.TableNumber`)))))))

(event `self.ReceiveBeginPlay`
  ;[1 1 1] Get Reference to Bar
  (bind _returnvalue (`GameplayStatics.GetActorOfClass` "/Game/BluePrints/Tavern_Logic/BP_Bar.BP_Bar_C"))
  (set `self.BarReference` _returnvalue)
  ;[1 1 1] Create Dialogue widget
  (bind _returnvalue_2 (`|CreateWidget` "/Game/BluePrints/UI/ChatUI/WB_TableInteraction.WB_TableInteraction_C" (`GameplayStatics.GetPlayerController` 0)))
  (set `self.DialogueWidget` _returnvalue_2))

(event `ContinueTimers`
  (for _array_element (`self.TimerHandels`)
    (`KismetSystemLibrary.K2_UnPauseTimerHandle` _array_element)))

(event `PauseTimers`
  (for _array_element (`self.TimerHandels`)
    (`KismetSystemLibrary.K2_PauseTimerHandle` _array_element)))

(event `self.rerer.OnBeginCursorOver`
  (params (TouchedComponent :type "PrimitiveComponent Object Reference"))
  ;[1 1 1] Interaction Logic
  (if (`/Game/BluePrints/ActorComponents/Interactable.Active` (`self.Interactable`))
    (`/Game/BluePrints/FunctionLists/FL_Interactable.Highlighted` (`self.DefaultSceneRoot`))))

(event `self.rerer.OnEndCursorOver`
  (params (TouchedComponent :type "PrimitiveComponent Object Reference"))
  ;[1 1 1] Interaction Logic
  (if (`/Game/BluePrints/ActorComponents/Interactable.Active` (`self.Interactable`))
    (`/Game/BluePrints/FunctionLists/FL_Interactable.DeHighlight` (`self.DefaultSceneRoot`))))

(event `Drinking`
  ;[1 1 1] Activate the Customers drinking and leaving after some time
  (bind _returnvalue (`KismetSystemLibrary.K2_SetTimerDelegate` (delegate `DrinkingTimer`) 10.0))
  (`KismetArrayLibrary.Array_Add` (`self.TimerHandels`) _returnvalue))

(event `DrinkingTimer`
  ;[1 1 1] Activate the Customers drinking and leaving after some time
  (bind _returnvalue (`GameplayStatics.GetActorOfClass` "/Game/BluePrints/GameManaging/BP_TavernManager.BP_TavernManager_C"))
  (`/Game/BluePrints/GameManaging/BP_TavernManager.EmptyOutTable` _returnvalue (`self.TableNumber`)))

(event `self.Interactable.DInteract`
  (bind _dialoguewidget (`self.DialogueWidget`))
  (`self.PauseTimers`)
  (add `/Game/BluePrints/UI/ChatUI/WB_TableInteraction.OnExit` _dialoguewidget (delegate `OnExit`))
  (`UserWidget.AddToViewport` _dialoguewidget 0)
  (`WidgetBlueprintLibrary.SetInputMode_UIOnlyEx` (`GameplayStatics.GetPlayerController` 0) _dialoguewidget)
  ;[1 1 1] Sets Current table reference if parent is Table
  (set `/Game/BluePrints/UI/ChatUI/WB_TableInteraction.CurrentTable` self (`self.DialogueWidget`)))

(event `OnExit`
  (`Widget.RemoveFromParent` (`self.DialogueWidget`))
  (`WidgetBlueprintLibrary.SetInputMode_GameAndUIEx` (`GameplayStatics.GetPlayerController` 0) null "DoNotLock" false)
  (`self.ContinueTimers`))

(fn `ChangeIndicator`
  (params (Waiting :type Boolean) (Order :type Boolean) (Leaving :type Boolean))
  (`SceneComponent.SetVisibility` (`self.Order_WorldUI`) Order false)
  (`SceneComponent.SetVisibility` (`self.LeavingIndicator`) Leaving false)
  (`SceneComponent.SetVisibility` (`self.WaitingUI`) Waiting false))

(fn `ClearTable`
  (bind _timerhandels (`self.TimerHandels`))
  (`self.DisableDrinks`)
  (set `self.OpenToChat` false)
  (`self.SetAvailability` true)
  (for _array_element (`self.NPCList`)
    (`/Game/BluePrints/Tavern_Logic/AI_Tavern/BP_AIcharacter.Leave` _array_element))
  (if (`self.Served`)
    ;[1 1 1] When served gain money
    (bind _gameinstance (`/Game/BluePrints/FunctionLists/Functions.GetCustomGameInstance`))
    (bind _reward (`/Game/BluePrints/GameManaging/BP_GameInstance.GetRewardReputation` _gameinstance))
    (`/Game/BluePrints/FunctionLists/Functions.EditReputation` _reward)
    (bind _rewardvalue (`self.GetOrderReward`))
    (`/Game/BluePrints/FunctionLists/Functions.EditMoneyReward` _rewardvalue)
    ;[1 1 1] Comment
    (set `self.Served` false)
    (else
      ;[1 1 1] When not served lower reputation
      (bind _gameinstance_2 (`/Game/BluePrints/FunctionLists/Functions.GetCustomGameInstance`))
      (bind _reward_2 (`/Game/BluePrints/GameManaging/BP_GameInstance.GetRewardReputation` _gameinstance_2))
      (`/Game/BluePrints/FunctionLists/Functions.EditReputation` (* _reward_2 -1))))
  (for _array_element_2 _timerhandels
    (`KismetSystemLibrary.K2_ClearAndInvalidateTimerHandle` _array_element_2)
    (`KismetArrayLibrary.Array_Clear` (`self.Order`)))
  (`KismetArrayLibrary.Array_Clear` _timerhandels)
  (`self.ChangeIndicator` false)
  (`KismetArrayLibrary.Array_Clear` (`self.NPCList`)))

(fn `DisableDrinks`
  (for _array_element (`|MakeArray` (`self.Cup1`) (`self.Cup2`) (`self.Cup3`) (`self.Cup`))
    (`SceneComponent.SetVisibility` _array_element false false)))

(fn `Enabledrinks`
  (for _index (range (`KismetArrayLibrary.Array_Length` (`self.NPCList`)))
    (`SceneComponent.SetVisibility` (`|GetArrayItem` (`|MakeArray` (`self.Cup1`) (`self.Cup2`) (`self.Cup3`) (`self.Cup`)) _index) true false)))

(fn `GetOrderReward`
  (returns (RewardValue :type Integer))
  (locals (Reward :type Integer))
  (set `local.Reward` 0)
  (bind _inventory (`/Game/BluePrints/FunctionLists/Functions.GetTavernInventory`))
  (for _array_element (`self.Order`)
    (bind _drink (`/Game/BluePrints/ActorComponents/DrinksAndIngredientsInventory.FindDrinkFromName` _inventory _array_element))
    (set `local.Reward` (+ (`local.Reward`) (`.Reward_23_24541ACE47FDAF4DE3B4C7B630DC12AA` (break `/Game/BluePrints/Drinks/Struct_Drinks` _drink)))))
  (return (`local.Reward`)))

(fn `GetSitLocation`
  (params (Index :type Integer))
  (returns (Location :type "SceneComponent Object Reference"))
  (switch `int` Index
    (:`0`
      (return (`self.AILocation_1`)))
    (:`1`
      (return (`self.AILocation_2`)))
    (:`2`
      (return (`self.AILocation_3`)))
    (:`3`
      (return (`self.AILocation_4`)))))

(fn `OrderStatusTimer`)

(fn `RemoveUI`
  (`Widget.RemoveFromParent` (`self.DialogueWidget`)))

(fn `UserConstructionScript`)