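; Tavern quest desk interactable that opens the main quests screen.
; BeginPlay creates the WB_MainQuests widget; interacting adds it to the viewport and switches input to UI only, and cursor hover toggles the highlight.
; A CheckActive macro passes only when the game state is CLOSED, but its uses are unwired, so nothing is gated.
; GoOnQuest is empty and GenerateNewQuest only adds an unset entry to SideQuests.
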(event `self.ReceiveBeginPlay`
  (bind _returnvalue (`|CreateWidget` "/Game/BluePrints/UI/QuestOverview/WB_MainQuests.WB_MainQuests_C"))
  (set `self.QuestWidget` _returnvalue))

(event `self.CheckInteraction.OnBeginCursorOver`
  (params (TouchedComponent :type "PrimitiveComponent Object Reference"))
  (`/Game/BluePrints/FunctionLists/FL_Interactable.Highlighted` (`self.SharedRoot`)))

(event `self.CheckInteraction.OnEndCursorOver`
  (params (TouchedComponent :type "PrimitiveComponent Object Reference"))
  (`/Game/BluePrints/FunctionLists/FL_Interactable.DeHighlight` (`self.SharedRoot`)))

(event `self.Interactable.DInteract`
  (`UserWidget.AddToViewport` (`self.QuestWidget`) 0)
  (`WidgetBlueprintLibrary.SetInputMode_UIOnlyEx` (`GameplayStatics.GetPlayerController` 0) null))

(fn `GenerateNewQuest`
  (`KismetArrayLibrary.Array_Add` (`self.SideQuests`)))

(fn `GoOnQuest`)

(fn `UserConstructionScript`)