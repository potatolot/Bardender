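; BP_Bar is the interactable tavern bar, opening either drink preparation or order serving based on the game state.
; BeginPlay creates both widgets, passing the tavern manager to serving and itself to preparation, and cursor hover toggles highlighting.
; Interacting while PREPARING or OPEN shows the matching widget, switches to UI-only input and stops player movement, with serving also fetching orders.
; An older PreparationMode branch and a StartTutorial call remain unconnected.
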(event `self.ReceiveBeginPlay`
  (bind _returnvalue (`|CreateWidget` "/Game/BluePrints/UI/BarUI/ServingUI/WB_Bar_Serving.WB_Bar_Serving_C" (`GameplayStatics.GetPlayerController` 0)))
  (bind _output_get (set `self.ServeWidget` _returnvalue))
  (bind _returnvalue_2 (`GameplayStatics.GetActorOfClass` "/Game/BluePrints/GameManaging/BP_TavernManager.BP_TavernManager_C"))
  (set `/Game/BluePrints/UI/BarUI/ServingUI/WB_Bar_Serving.TavernManagerRef` _returnvalue_2 _output_get)
  (bind _returnvalue_3 (`|CreateWidget` "/Game/BluePrints/UI/BarUI/WB_Bar_Preparation_Drinks.WB_Bar_Preparation_Drinks_C" (`GameplayStatics.GetPlayerController` 0)))
  (bind _output_get_2 (set `self.PreparationWidget` _returnvalue_3))
  (set `/Game/BluePrints/UI/BarUI/WB_Bar_Preparation_Drinks.BarReference` self _output_get_2))

(event `self.BarMesh.OnBeginCursorOver`
  (params (TouchedComponent :type "PrimitiveComponent Object Reference"))
  (`/Game/BluePrints/FunctionLists/FL_Interactable.Highlighted` (`self.DefaultSceneRoot`)))

(event `self.BarMesh.OnEndCursorOver`
  (params (TouchedComponent :type "PrimitiveComponent Object Reference"))
  (`/Game/BluePrints/FunctionLists/FL_Interactable.DeHighlight` (`self.DefaultSceneRoot`)))

(event `self.Interactable.DInteract`
  (bind _returnvalue (`GameplayStatics.GetPlayerController` 0))
  (bind _returnvalue_2 (`GameplayStatics.GetPlayerController` 0))
  (bind _servewidget (`self.ServeWidget`))
  (bind _gameinstance (`/Game/BluePrints/FunctionLists/Global_Functions.GetCustomGameInstance`))
  (switch `/Game/BluePrints/GameManaging/EGameState` (`/Game/BluePrints/GameManaging/BP_GameInstance.GameState` _gameinstance)
    (:`NewEnumerator0`
      ;[1 1 1] Preparation Logic
      (`UserWidget.AddToViewport` (`self.PreparationWidget`) 0)
      (`WidgetBlueprintLibrary.SetInputMode_UIOnlyEx` _returnvalue null)
      (`Controller.StopMovement` _returnvalue)
      (if (`self.TutorialCompleted`)
        _))
    (:`NewEnumerator1`
      (`UserWidget.AddToViewport` _servewidget 0)
      (`WidgetBlueprintLibrary.SetInputMode_UIOnlyEx` _returnvalue_2 _servewidget)
      (`Controller.StopMovement` _returnvalue_2)
      (`/Game/BluePrints/UI/BarUI/ServingUI/WB_Bar_Serving.GetOrders` _servewidget))))

(fn `UserConstructionScript`)