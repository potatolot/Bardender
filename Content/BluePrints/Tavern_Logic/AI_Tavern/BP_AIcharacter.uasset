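; Tavern AI character that can walk to a spot, report a seat location and flag itself as seated.
; MoveTowards sends its controller to a hard-coded world point, while GetSitLocation separately returns the first sit location of the referenced table.
; The SitDown event only sets the SitsDown flag.
; It looks unfinished: SetColor just prints a debug string, and the montage and material calls are disconnected.
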(event `SitDown`
  (set `self.SitsDown` true))

(event `self.ReceiveTick`
  (params (DeltaSeconds :type "Float (single-precision)")))

(event `self.ReceiveBeginPlay`)

(fn `GetSitLocation`
  (returns (Location :type "Vector Structure"))
  (return (`|GetArrayItem` (`/Game/BluePrints/Tavern_Logic/BP_Table.SitLocations` (`self.TableRef`)))))

(fn `MoveTowards`
  (`AIBlueprintHelperLibrary.SimpleMoveToLocation` (`self.GetController` self) (`KismetMathLibrary.MakeVector` 870.0 210.0 74.0)))

(fn `SetColor`
  (`KismetSystemLibrary.PrintString` "Color Change"))

(fn `UserConstructionScript`)