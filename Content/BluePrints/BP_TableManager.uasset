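; Table manager that seats groups of AI customer characters at free tables on a randomized timer.
; While enabled with tables free, a Delay on Tick drives a roughly once-per-second counter that triggers spawning and rerolls the next interval.
; Each small random group spawns at SpawnPoint and moves to seat offsets on one random table.
; That table is then marked unavailable and removed from the pool, with no re-adding here.
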(event `self.ReceiveBeginPlay`
  (set `self.AvailableTables` (`self.Tables`)))

(event `self.ReceiveTick`
  (params (DeltaSeconds :type "Float (single-precision)"))
  (if (`self.Enabled`)
    (if (> (`KismetArrayLibrary.Array_Length` (`self.AvailableTables`)) 0)
      (`KismetSystemLibrary.Delay` 1.0)
      (bind _result (`/Engine/EditorBlueprintResources/StandardMacros.IncrementInt` (`self.RandomTimer`))
        (:`  `
          (if (== _result (`self.SpawnTime`))
            (`self.SetRandomSpawnTime`)
            (`self.SpawnNewGroup`)
            (set `self.RandomTimer` 0)))))))

(fn `SetRandomSpawnTime`
  (set `self.SpawnTime` (`KismetMathLibrary.RandomIntegerInRange` 2 5)))

(fn `SpawnNewGroup`
  (bind _availabletables (`self.AvailableTables`))
  (bind _output_get (set `self.RandomTable` (`KismetMathLibrary.RandomIntegerInRange` 0 (- (`KismetArrayLibrary.Array_Length` (`self.AvailableTables`)) 1))))
  (`KismetArrayLibrary.Array_Clear` (`self.AICharacters`))
  (for _index (range (+ (`KismetMathLibrary.RandomIntegerInRange` 1 3) 1))
    ;[1 1 1] TO DO: Spawn amount of new ai characters at spawnpoint
    (bind _returnvalue (`|SpawnActorFromClass` "/Game/BluePrints/AI_Tavern/BP_AIcharacter.BP_AIcharacter_C" (`self.GetTransform` (`self.SpawnPoint`)) "Undefined" "OverrideRootScale" null null))
    (`KismetArrayLibrary.Array_Add` (`self.AICharacters`) _returnvalue)
    (bind _output (`|GetArrayItem` _availabletables _output_get))
    (`/Game/BluePrints/AI_Tavern/BP_AIcharacter.MoveToTable` _returnvalue (+ (`|GetArrayItem` (`/Game/BluePrints/BP_Table.SitLocations` _output) _index) (`SceneComponent.K2_GetComponentLocation` (`/Game/BluePrints/BP_Table.DefaultSceneRoot` _output)))))
  (`/Game/BluePrints/BP_Table.SetAvailability` _output false)
  (`KismetArrayLibrary.Array_RemoveItem` _availabletables _output))

(fn `UserConstructionScript`)