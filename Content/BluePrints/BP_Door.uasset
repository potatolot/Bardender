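; BP_Door is an interactable door that opens a UI widget when used.
; Cursor hover over its Box highlights and un-highlights the door through DefaultSceneRoot, only while its Interactable component is active.
; It creates a WB_DoorUI widget at BeginPlay, and the Interactable's DInteract event adds it to the viewport, switches to UI-only input and sets the Open flag.
; The file contains no door movement logic.
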(event `self.Box.OnBeginCursorOver`
  (params (TouchedComponent :type "PrimitiveComponent Object Reference"))
  (if (`/Game/BluePrints/ActorComponents/Interactable.Active` (`self.Interactable`))
    (`/Game/BluePrints/FunctionLists/FL_Interactable.Highlighted` (`self.DefaultSceneRoot`))))

(event `self.Box.OnEndCursorOver`
  (params (TouchedComponent :type "PrimitiveComponent Object Reference"))
  (if (`/Game/BluePrints/ActorComponents/Interactable.Active` (`self.Interactable`))
    (`/Game/BluePrints/FunctionLists/FL_Interactable.DeHighlight` (`self.DefaultSceneRoot`))))

(event `self.ReceiveBeginPlay`
  (bind _returnvalue (`|CreateWidget` "/Game/BluePrints/UI/WB_DoorUI.WB_DoorUI_C"))
  (set `self.DoorWidget` _returnvalue))

(event `self.Interactable.DInteract`
  (`UserWidget.AddToViewport` (`self.DoorWidget`) 0)
  (`WidgetBlueprintLibrary.SetInputMode_UIOnlyEx` (`GameplayStatics.GetPlayerController` 0) null)
  (set `self.Open` true))

(fn `UserConstructionScript`)