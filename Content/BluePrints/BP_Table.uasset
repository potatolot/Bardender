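; Tavern table actor that customers order from, with a bobbing, spinning world-space order icon shown while it is ready to order.
; SetAvailability toggles the interactable and icon; OnSetupTable is meant to randomize an order, but its loop is empty.
; Cursor hover highlights the active table, and interacting opens a dialogue widget in UI-only input until exit.
; OnOrder updates the tavern UI, clears the icon and adds the order to the player's inventory.
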(event `self.ReceiveTick`
  (params (DeltaSeconds :type "Float (single-precision)"))
  (bind _returnvalue (`self.GetGameTimeSinceCreation`))
  (bind _order_worldui (`self.Order_WorldUI`))
  (bind (_returnvalue_x _returnvalue_y _returnvalue_z) (`KismetMathLibrary.BreakVector` (`SceneComponent.K2_GetComponentLocation` _order_worldui)))
  (`SceneComponent.K2_SetWorldLocation` _order_worldui (`KismetMathLibrary.MakeVector` _returnvalue_x _returnvalue_y (+ (* (`KismetMathLibrary.DegSin` (* _returnvalue (`self.OrderIcon_Speed`))) (`self.OrderIcon_Distance`)) _returnvalue_z)) false false)
  (`SceneComponent.K2_SetRelativeRotation` _order_worldui (`KismetMathLibrary.Conv_VectorToRotator` (`KismetMathLibrary.CreateVectorFromYawPitch` (* (`self.OrderIcon_RotationSpeed`) _returnvalue))) false false))

(event `SetAvailability`
  (params (newAvailability :type Boolean))
  (bind _returnvalue (not newAvailability))
  (set `/Game/BluePrints/ActorComponents/Interactable.Active` _returnvalue (`self.Interactable`))
  (if true
    (`self.OnSetupTable` 0)
    (`self.SetReadyToOrder` _returnvalue)))

(event `OnSetupTable`
  (params (Customers :type Integer))
  ;[1 1 1] Generate a random order
  (for _ (range (+ Customers 1))
    _))

(event `OnOrder`
  ;[1 1 1] Add order to the UI
  (bind _foundwidgets (`WidgetBlueprintLibrary.GetAllWidgetsOfClass` "/Game/BluePrints/UI/WB_TavernUI.WB_TavernUI_C"))
  (`/Game/BluePrints/UI/WB_TavernUI.Addorder` (`|GetArrayItem` _foundwidgets))
  (`self.SetReadyToOrder` false)
  ;[1 1 1] Add order to players inventory
  (bind _asbp_character (cast `/Game/BluePrints/Character_BP/BP_Character` (`GameplayStatics.GetPlayerCharacter` 0)))
  (`/Game/BluePrints/ActorComponents/Inventory.AddOrder` (`/Game/BluePrints/Character_BP/BP_Character.Inventory` _asbp_character) (`self.Order`)))

(event `self.ReceiveBeginPlay`
  ;[1 1 1] Create Dialogue widget
  (bind _returnvalue (`|CreateWidget` "/Game/BluePrints/UI/WB_Dialogue.WB_Dialogue_C" (`GameplayStatics.GetPlayerController` 0)))
  (set `self.DialogueUI` _returnvalue))

(event `self.rerer.OnBeginCursorOver`
  (params (TouchedComponent :type "PrimitiveComponent Object Reference"))
  (if (`/Game/BluePrints/ActorComponents/Interactable.Active` (`self.Interactable`))
    (`/Game/BluePrints/FunctionLists/FL_Interactable.Highlighted` (`self.DefaultSceneRoot`))))

(event `self.rerer.OnEndCursorOver`
  (params (TouchedComponent :type "PrimitiveComponent Object Reference"))
  (if (`/Game/BluePrints/ActorComponents/Interactable.Active` (`self.Interactable`))
    (`/Game/BluePrints/FunctionLists/FL_Interactable.DeHighlight` (`self.DefaultSceneRoot`))))

(event `self.Interactable.DInteract`
  (bind _dialogueui (`self.DialogueUI`))
  (add `/Game/BluePrints/UI/WB_Dialogue.OnExit` _dialogueui (delegate `OnExit`))
  (`UserWidget.AddToViewport` _dialogueui 0)
  (`WidgetBlueprintLibrary.SetInputMode_UIOnlyEx` (`GameplayStatics.GetPlayerController` 0) _dialogueui)
  ;[1 1 1] Sets Current table reference if parent is Table
  (set `/Game/BluePrints/UI/WB_Dialogue.CurrentTable` self (`self.DialogueUI`)))

(event `OnExit`
  (`Widget.RemoveFromParent` (`self.DialogueUI`))
  (`WidgetBlueprintLibrary.SetInputMode_GameAndUIEx` (`GameplayStatics.GetPlayerController` 0) null "DoNotLock" false))

(fn `RemoveUI`
  (`Widget.RemoveFromParent` (`self.DialogueUI`)))

(fn `SetReadyToOrder`
  (params (Value :type Boolean))
  (`SceneComponent.SetVisibility` (`self.Order_WorldUI`) Value false)
  (set `self.ReadyToOrder` Value))

(fn `UserConstructionScript`)