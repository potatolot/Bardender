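; BP_Wall is a wall actor that shows or hides its static mesh according to the player camera's horizontal facing.
; On BeginPlay it caches Camera1 from the player's BP_Character.
; Each Tick it dots the flattened camera forward with the mesh's right vector, showing the mesh only when the result is below Min and above Max, despite those names.
; Hide and UnHide events toggle visibility without affecting child components.
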(event `self.ReceiveBeginPlay`
  (bind _asbp_character (cast `/Game/BluePrints/Character_BP/BP_Character` (`GameplayStatics.GetPlayerCharacter` 0)))
  (set `self.Camera` (`/Game/BluePrints/Character_BP/BP_Character.Camera1` _asbp_character)))

(event `self.ReceiveTick`
  (params (DeltaSeconds :type "Float (single-precision)"))
  (bind _returnvalue (`KismetMathLibrary.Dot_VectorVector` (`KismetMathLibrary.Normal` (`KismetMathLibrary.MakeVector` (.x (`SceneComponent.GetForwardVector` (`self.Camera`))) (.y (`SceneComponent.GetForwardVector` (`self.Camera`))))) (`KismetMathLibrary.Normal` (`SceneComponent.GetRightVector` (`self.StaticMeshComponent`)))))
  (if (and (< _returnvalue (`self.Min`)) (> _returnvalue (`self.Max`)))
    (`self.UnHide`)
    (else
      (`self.Hide`))))

(event `Hide`
  (`SceneComponent.SetVisibility` (`self.StaticMeshComponent`) false false))

(event `UnHide`
  (`SceneComponent.SetVisibility` (`self.StaticMeshComponent`) true false))

(fn `UserConstructionScript`)